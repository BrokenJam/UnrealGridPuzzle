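; Puzzle interactable that launches its Sphere component and shows an interact HUD when the player is near.
; While IsLaunch is true, Tick applies a constant upward force to Sphere; nothing in this graph sets that flag.
; BeginPlay creates a BP_HUD widget, which Sphere1 overlaps add to or remove from the viewport for the player character, toggling the mouse cursor with it.
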(event `self.ReceiveTick`
  (params (DeltaSeconds :type "Float (single-precision)"))
  (if (`self.isLaunch`)
    (`PrimitiveComponent.AddForce` (`self.Sphere`) (0.0 0.0 2000.0) "None" false)))

(event `self.ReceiveBeginPlay`
  ; Interact Prompt on HUD
  (bind _returnvalue (`|CreateWidget` "/Game/Interactables/PuzzleUI/BP_HUD.BP_HUD_C"))
  (set `self.Interact` _returnvalue))

(event `self.Sphere1.OnComponentBeginOverlap`
  (params (OverlappedComponent :type "PrimitiveComponent Object Reference") (OtherActor :type "Actor Object Reference") (OtherComp :type "PrimitiveComponent Object Reference") (OtherBodyIndex :type Integer) (bFromSweep :type Boolean) (SweepResult :type "HitResult Structure (by ref)"))
  ; Interact Prompt on HUD
  (if (== OtherActor (`GameplayStatics.GetPlayerCharacter` 0))
    (`UserWidget.AddToViewport` (`self.Interact`) 0)
    (set `PlayerController.bShowMouseCursor` true (`GameplayStatics.GetPlayerController` 0))))

(event `self.Sphere1.OnComponentEndOverlap`
  (params (OverlappedComponent :type "PrimitiveComponent Object Reference") (OtherActor :type "Actor Object Reference") (OtherComp :type "PrimitiveComponent Object Reference") (OtherBodyIndex :type Integer))
  ; Interact Prompt on HUD
  (if (== OtherActor (`GameplayStatics.GetPlayerCharacter` 0))
    (`Widget.RemoveFromParent` (`self.Interact`))
    (set `PlayerController.bShowMouseCursor` false (`GameplayStatics.GetPlayerController` 0))))

(fn `UserConstructionScript`)